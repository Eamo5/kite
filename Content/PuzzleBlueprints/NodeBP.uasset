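; NodeBP is a puzzle node that changes to a selected material when overlapped and controls which linked node can be triggered next.
; An overlap disables the node's collision, then enables query collision on its next or previous neighbor according to its Direction flag.
; Starting at the first or last node sets forward or backward mode and disables the opposite end's collision.
; Forward mode also passes the flag along to each next node.
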(event `self.ReceiveActorBeginOverlap`
  (params (OtherActor :type "Actor Object Reference"))
  (bind _nextnode (`self.NextNode`))
  (bind _prevnode (`self.PrevNode`))
  (`PrimitiveComponent.SetMaterial` (`self.Sph_mesh`) 0 "/Game/PuzzleBlueprints/NodeSelectedMat.NodeSelectedMat")
  (`PrimitiveComponent.SetCollisionEnabled` (`self.ParentNode`) "NoCollision")
  (if (`self.First`)
    (set `/Game/PuzzleBlueprints/NodeBP.Direction` true (`self.NextNode`)) ; Also set the next node's direction
    (set `self.Direction` true) ; Direction set to 'true' will mean the puzzle is set to 'forward' mode
    (`PrimitiveComponent.SetCollisionEnabled` (`/Game/PuzzleBlueprints/NodeBP.ParentNode` (`self.LastNode`)) "NoCollision")
    (elif (`self.Last`)
      (set `self.Direction` false) ; Direction set to 'false' will mean the puzzle is set to 'backward' mode
      (set `/Game/PuzzleBlueprints/NodeBP.Direction` false (`self.PrevNode`)) ; Set prev node's direction
      (`PrimitiveComponent.SetCollisionEnabled` (`/Game/PuzzleBlueprints/NodeBP.ParentNode` (`self.FirstNode`)) "NoCollision")))
  (if (`self.Direction`)
    (if (`KismetSystemLibrary.IsValidSoftObjectReference` (`|ConvertAsset` _nextnode))
      (`PrimitiveComponent.SetCollisionEnabled` (`/Game/PuzzleBlueprints/NodeBP.ParentNode` _nextnode) "QueryOnly")
      (set `/Game/PuzzleBlueprints/NodeBP.Direction` true (`self.NextNode`)))
    (elif (`KismetSystemLibrary.IsValidSoftObjectReference` (`|ConvertAsset` _prevnode))
      (`PrimitiveComponent.SetCollisionEnabled` (`/Game/PuzzleBlueprints/NodeBP.ParentNode` _prevnode) "QueryOnly"))))

(fn `UserConstructionScript`)