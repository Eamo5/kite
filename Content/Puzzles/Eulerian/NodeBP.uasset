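; Node in an Eulerian path puzzle that the player traverses by overlapping linked nodes in order from either end.
; The end node touched first sets forward or backward direction, flags the opposite end as the finish and disables its collision.
; Each overlap marks the node selected, disables its collision, then enables and highlights the neighbor in that direction.
; Overlapping the opposite end applies the puzzle-complete material.
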(event `self.ReceiveActorBeginOverlap`
  (params (OtherActor :type "Actor Object Reference"))
  (bind _nextnode (`self.NextNode`))
  (bind _nextnode_2 (`self.NextNode`))
  (bind _prevnode (`self.PrevNode`))
  (`PrimitiveComponent.SetMaterial` (`self.node`) 0 "/Game/Puzzles/Eulerian/NodeSelectedMat.NodeSelectedMat")
  (`PrimitiveComponent.SetCollisionEnabled` (`self.ParentNode`) "NoCollision")
  (if (`self.FirstStart`)
    (if (`self.Last`)
      (`PrimitiveComponent.SetMaterial` (`self.node`) 0 "/Game/Puzzles/Eulerian/PuzzleComplete.PuzzleComplete"))
    (elif (`self.LastStart`)
      (if (`self.First`)
        (`PrimitiveComponent.SetMaterial` (`self.node`) 0 "/Game/Puzzles/Eulerian/PuzzleComplete.PuzzleComplete"))
      (else
        (if (`self.First`)
          (set `self.FirstStart` true)
          (set `/Game/Puzzles/Eulerian/NodeBP.FirstStart` true (`self.LastNode`))
          (set `/Game/Puzzles/Eulerian/NodeBP.Direction` true (`self.NextNode`)) ; Also set the next node's direction
          (set `self.Direction` true) ; Direction set to 'true' will mean the puzzle is set to 'forward' mode
          (`PrimitiveComponent.SetCollisionEnabled` (`/Game/Puzzles/Eulerian/NodeBP.ParentNode` (`self.LastNode`)) "NoCollision")
          (elif (`self.Last`)
            (set `self.LastStart` true)
            (set `/Game/Puzzles/Eulerian/NodeBP.LastStart` true (`self.FirstNode`))
            (set `self.Direction` false) ; Direction set to 'false' will mean the puzzle is set to 'backward' mode
            (set `/Game/Puzzles/Eulerian/NodeBP.Direction` false (`self.PrevNode`)) ; Set prev node's direction
            (`PrimitiveComponent.SetCollisionEnabled` (`/Game/Puzzles/Eulerian/NodeBP.ParentNode` (`self.FirstNode`)) "NoCollision")))
        (if (`self.Direction`)
          (if (`KismetSystemLibrary.IsValidSoftObjectReference` (`|ConvertAsset` _nextnode_2))
            (`PrimitiveComponent.SetCollisionEnabled` (`/Game/Puzzles/Eulerian/NodeBP.ParentNode` _nextnode_2) "QueryOnly")
            (set `/Game/Puzzles/Eulerian/NodeBP.Direction` true _nextnode)
            (`PrimitiveComponent.SetMaterial` (`/Game/Puzzles/Eulerian/NodeBP.node` _nextnode) 0 "/Game/Puzzles/Eulerian/NextNode.NextNode"))
          (elif (`KismetSystemLibrary.IsValidSoftObjectReference` (`|ConvertAsset` _prevnode))
            (`PrimitiveComponent.SetCollisionEnabled` (`/Game/Puzzles/Eulerian/NodeBP.ParentNode` _prevnode) "QueryOnly")
            (`PrimitiveComponent.SetMaterial` (`/Game/Puzzles/Eulerian/NodeBP.node` (`self.PrevNode`)) 0 "/Game/Puzzles/Eulerian/NextNode.NextNode")))))))

(fn `UserConstructionScript`)