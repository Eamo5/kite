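; Audio trigger Blueprint that, going by its name, plays lightning sound along a spline for the kite pawn.
; A box overlap that passes the KitePawnV1 casts calls FadeOut on any playing audio, restarts it from an offset, then starts MoveAudio.
; MoveAudio re-calls itself after a short Delay, keeping an Arrow just above the spline point closest to the pawn.
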(event `self.Box.OnComponentBeginOverlap`
  (params (OverlappedComponent :type "PrimitiveComponent Object Reference") (OtherActor :type "Actor Object Reference") (OtherComp :type "PrimitiveComponent Object Reference") (OtherBodyIndex :type Integer) (bFromSweep :type Boolean) (SweepResult :type "HitResult Structure (by ref)"))
  (bind _audio (`self.Audio`))
  (castclass `/Game/Characters/KitePawnV1` (`GameplayStatics.GetObjectClass` OtherActor))
  (if (`AudioComponent.IsPlaying` _audio)
    (`AudioComponent.FadeOut` (`self.Audio`) 30.0 0.0 "Linear"))
  (`AudioComponent.Play` _audio 5.0)
  (castclass `/Game/Characters/KitePawnV1` (`GameplayStatics.GetObjectClass` (`GameplayStatics.GetPlayerCharacter` 0)))
  (`self.MoveAudio`))

(event `MoveAudio`
  (bind (_returnvalue_x _returnvalue_y _returnvalue_z) (`KismetMathLibrary.BreakVector` (`SplineComponent.FindLocationClosestToWorldLocation` (`self.Spline`) (`self.K2_GetActorLocation` (`self.Kite Pawn V1_Reference`)) "World")))
  (`SceneComponent.K2_SetWorldLocation` (`self.Arrow`) (`KismetMathLibrary.MakeVector` _returnvalue_x _returnvalue_y (+ _returnvalue_z 50.0)) false false)
  (`KismetSystemLibrary.Delay` 0.05)
  (`self.MoveAudio`))

(fn `UserConstructionScript`)