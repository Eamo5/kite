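; SoundscapeTrigger_BP is a sphere trigger that switches ambient Soundscape palette content as actors enter and leave its area.
; On BeginPlay it derives the collection name from its SoundscapeState gameplay tag.
; Entering registers the palette collection with the Soundscape subsystem and sets that state, with an optional debug print.
; Leaving only removes the collection, as the ClearState call and its debug print are unconnected.
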(event `self.ReceiveBeginPlay`
  (set `self.Palette Collection Name` (`BlueprintGameplayTagLibrary.GetTagName` (`self.Soundscape State`))))

(event `self.ReceiveActorBeginOverlap`
  (params (OtherActor :type "Actor Object Reference")))

(event `self.Sphere.OnComponentBeginOverlap`
  (params (OverlappedComponent :type "PrimitiveComponent Object Reference") (OtherActor :type "Actor Object Reference") (OtherComp :type "PrimitiveComponent Object Reference") (OtherBodyIndex :type Integer) (bFromSweep :type Boolean) (SweepResult :type "HitResult Structure (by ref)"))
  (bind _returnvalue (subsystem `SoundscapeSubsystem`))
  (`SoundscapeSubsystem.AddPaletteCollection` _returnvalue (`self.Palette Collection Name`) (`self.Palette Collection`))
  (`SoundscapeSubsystem.SetState` _returnvalue (`self.Soundscape State`))
  (if (`self.Debug Trigger`)
    (`KismetSystemLibrary.PrintString` (`KismetTextLibrary.Conv_TextToString` (`|FormatText` (`KismetTextLibrary.Conv_NameToText` (`self.Palette Collection Name`)))) true true (struct :`R` 1.0 :`G` 0.296536 :`A` 1.0) 20.0)))

(event `self.Sphere.OnComponentEndOverlap`
  (params (OverlappedComponent :type "PrimitiveComponent Object Reference") (OtherActor :type "Actor Object Reference") (OtherComp :type "PrimitiveComponent Object Reference") (OtherBodyIndex :type Integer))
  (`SoundscapeSubsystem.RemovePaletteCollection` (subsystem `SoundscapeSubsystem`) (`self.Palette Collection Name`)))

(fn `UserConstructionScript`)